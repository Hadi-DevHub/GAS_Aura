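; BP_FireBall is an ability actor for a boomerang-style fireball that flies forward, then returns to its instigator.
; On the authority only, an outgoing timeline lerps it from spawn to an apex set along its forward vector.
; A returning timeline then lerps it toward the instigator's live location.
; Once within MaxReturnDistance of the instigator, it calls OnHit and destroys itself.
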(event EventBeginPlay
  (bind _returnvalue (Game|GetInstigator))
  (bind _returnvalue_2 (Transformation|GetActorLocation))
  (bind _returnvalue_3 (Transformation|GetActorLocation _returnvalue))
  (if (Ability|HasAuthority)
    (Variables|Default|SetInitialLocation _returnvalue_2)
    (Variables|Default|SetApexDistance (+ _returnvalue_2 (* (Transformation|GetActorForwardVector) (Variables|Default|GetOutgoingDistanceMultiplier))))
    (bind _outgoingdistance (Timeline|OutgoingTimeline Play)
      (:Update
        (Transformation|SetActorLocation (Math|Vector|Lerp(Vector) (Variables|Default|GetInitialLocation) (Variables|Default|GetApexDistance) _outgoingdistance) false false))
      (:Finished
        (bind _returningtimeline (Timeline|ReturningTimeline Play)
          (:Update
            (Variables|Default|SetInstigatorLocation _returnvalue_3)
            (Transformation|SetActorLocation (Math|Vector|Lerp(Vector) (Variables|Default|GetApexDistance) _returnvalue_3 _returningtimeline) false false)
            (if (<= (Math|Vector|VectorLength (- (Variables|Default|GetInstigatorLocation) (Math|Vector|Lerp(Vector) (Variables|Default|GetApexDistance) _returnvalue_3 _returningtimeline))) (Variables|Default|GetMaxReturnDistance))
              (Class|AuraProjectile|OnHit)
              (Actor|DestroyActor))))))))

(event EventTick
  (params (DeltaSeconds :type Float%20%28single-precision%29)))

(fn ConstructionScript)