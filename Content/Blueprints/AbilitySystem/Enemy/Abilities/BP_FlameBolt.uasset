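; Flame bolt actor from the enemy ability set that removes itself once it stops moving.
; Each Tick it compares its location with the previous frame's, using a minimum-distance threshold to detect a stall rather than handling hit or overlap events.
; On a stall it spawns a tiny fire-fade Niagara effect, plays a fireball sound and destroys itself.
; This graph contains no movement or damage logic.
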(event EventBeginPlay)

(event Collision|EventActorBeginOverlap
  (params (OtherActor :type Actor%20Object%20Reference)))

(event EventTick
  (params (DeltaSeconds :type Float%20%28single-precision%29))
  (Variables|Default|SetActorLocationLastFrame (Variables|Default|GetActorLocationCurrentFrame))
  (Variables|Default|SetActorLocationCurrentFrame (Transformation|GetActorLocation))
  (if (< (Math|Vector|VectorLength (- (Variables|Default|GetActorLocationCurrentFrame) (Variables|Default|GetActorLocationLastFrame))) (Variables|Default|GetMinDistanceBetweenFrames))
    (Niagara|SpawnSystematLocation "/Game/Assets/Effects/Projectiles/FireExplosion/NS_FireFade.NS_FireFade" (Transformation|GetActorLocation) "0, 0, 0" "0.010000,0.010000,0.010000")
    (Audio|PlaySoundatLocation "/Game/Assets/Sounds/Abilities/FireBolt/wav/Shoot/SFX_FireBall_Shoot_LowLevel_02.SFX_FireBall_Shoot_LowLevel_02" (Transformation|GetActorLocation) "0, 0, 0" 1.0 1.0 0.0 0 0 0 0)
    (Actor|DestroyActor)))

(fn ConstructionScript)