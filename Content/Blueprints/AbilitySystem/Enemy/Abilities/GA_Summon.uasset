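; Enemy gameplay ability that summons random minions around the caster, using the Shaman summon montage.
; On activation it shuffles the spawn locations, starts the montage and plays ground Niagara effects at each location.
; The montage's Ability.Attack gameplay event starts a delayed loop that spawns AI-controlled minions one by one, facing away from the caster, then ends the ability.
; Each spawn and destruction updates the caster's minion count through a message.
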(event Custom|OnDestroyed_Event
  (params (DestroyedActor :type Actor%20Object%20Reference))
  (Class|CombatInterface|IncrementNumberOfMinions(Message) (Ability|GetAvatarActorfromActorInfo) -1))

(event Ability|EventActivateAbility
  (Variables|Default|SetSpawnIndex 0)
  (bind _returnvalue (Class|AuraSummonAbility|GetSpawnLocations))
  (bind _output_get (Variables|Default|SetSpawnLocations _returnvalue))
  (Utilities|Array|Shuffle _output_get)
  (|PlayMontageandWaitProxy "None" "/Game/Assets/Enemies/Shaman/Animations/AM_Shaman_Summon.AM_Shaman_Summon" 1.0 "None" true 1.0 0.0 false
    (:then
      (Ability|Tasks|WaitGameplayEvent "(TagName=\"Ability.Attack\")" 0
        (:then
          (for _array_element (Variables|Default|GetSpawnLocations)
            (Niagara|SpawnSystematLocation "/Game/Assets/Effects/Combat/NS_GroundSummon.NS_GroundSummon" _array_element)))
        (:EventReceived
          (if (< (Variables|Default|GetSpawnIndex) (Utilities|Array|Length (Variables|Default|GetSpawnLocations))) :!label _label
            (Utilities|FlowControl|Delay 0.2)
            (bind _returnvalue_2 (Game|SpawnActorfromClass (Class|AuraSummonAbility|GetRandomMinion) (Math|Transform|MakeTransform (+ (Utilities|Array|Get(acopy) (Variables|Default|GetSpawnLocations) (Variables|Default|GetSpawnIndex)) "0.000000,0.000000,70.000000") (Math|Rotator|FindLookatRotation (Transformation|GetActorLocation (Ability|GetAvatarActorfromActorInfo)) (+ (Utilities|Array|Get(acopy) (Variables|Default|GetSpawnLocations) (Variables|Default|GetSpawnIndex)) "0.000000,0.000000,70.000000")) "1.000000,1.000000,1.000000") "AlwaysSpawn" "MultiplyWithRoot" 0 0))
            (Game|AssignOnDestroyed _returnvalue_2 (delegate Custom|OnDestroyed_Event))
            (Pawn|SpawnDefaultController _returnvalue_2)
            (Class|CombatInterface|IncrementNumberOfMinions(Message) (Ability|GetAvatarActorfromActorInfo) 1)
            (Math|Integer|IncrementInt (Variables|Default|GetSpawnIndex)
              (:%20%20
                (goto _label)))
            (else
              (Ability|EndAbility))))))))

(event Ability|EventOnEndAbility
  (params (bWasCancelled :type Boolean)))