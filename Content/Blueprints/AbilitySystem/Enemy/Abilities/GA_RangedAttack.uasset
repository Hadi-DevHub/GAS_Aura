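; Enemy ranged attack gameplay ability that plays a random attack montage and fires a projectile at the combat target.
; On activation it turns the avatar toward the target and waits for the Montage.Attack.1 event to spawn the projectile.
; The random montage pick is re-evaluated for the socket tag, so the two can come from different entries.
; The ability ends when the montage completes, is interrupted or is cancelled.
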(event Ability|EventActivateAbility
  (bind _output_get (Variables|Default|SetThisCharacter (Ability|GetAvatarActorfromActorInfo)))
  (bind _ascombat_interface (Utilities|Casting|CastToCombatInterface _output_get))
  (Variables|Default|SetCombat%20Interface _ascombat_interface)
  (|PlayMontageandWaitProxy "None" (.AttackMontage (Utilities|Struct|BreakTaggedMontages (Class|AuraDamageGameplayAbility|GetRandomTaggedMontagesfromArray (Class|CombatInterface|GetAttackMontages (Variables|Default|GetCombat%20Interface))))) 1.0 "None" true 1.0 0.0 false
    (:then
      (Ability|Tasks|WaitGameplayEvent "(TagName=\"Montage.Attack.1\")" 0 true
        (:then
          (bind _returnvalue (Class|EnemyInterface|GetCombatTarget(Message) (Variables|Default|GetThisCharacter)))
          (Utilities|IsValid _returnvalue
            (:Is%20Valid
              (Class|CombatInterface|SetFacingTarget(Message) (Variables|Default|GetThisCharacter) (Transformation|GetActorLocation _returnvalue)))))
        (:EventReceived
          (Class|CombatInterface|GetCombatSocketLocation (Variables|Default|GetCombat%20Interface) (.MontageTag (Utilities|Struct|BreakTaggedMontages (Class|AuraDamageGameplayAbility|GetRandomTaggedMontagesfromArray (Class|CombatInterface|GetAttackMontages (Variables|Default|GetCombat%20Interface))))))
          (Class|AuraProjectileSpell|SpawnProjectile (Transformation|GetActorLocation _returnvalue) (.SocketTag (Utilities|Struct|BreakTaggedMontages (Class|AuraDamageGameplayAbility|GetRandomTaggedMontagesfromArray (Class|CombatInterface|GetAttackMontages (Variables|Default|GetCombat%20Interface)))))))))
    (:OnCompleted
      (Ability|EndAbility :!label _label))
    (:OnInterrupted
      (goto _label))
    (:OnCancelled
      (goto _label))))

(event Ability|EventOnEndAbility
  (params (bWasCancelled :type Boolean)))