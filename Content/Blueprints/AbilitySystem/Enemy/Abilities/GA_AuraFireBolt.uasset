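; Gameplay ability that casts Aura's Fire Bolt, spawning projectiles toward the target under the mouse cursor.
; On activation it commits, stores the hit location and actor from target data, and turns the avatar toward that location.
; A montage gameplay event triggers the spawn from the weapon socket, with overridden pitch and the hit actor as homing target.
; The ability ends only when the montage completes.
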(event Ability|EventActivateAbility
  (Ability|CommitAbility)
  (bind _data (|TargetDataUnderMouse)
    (:ValidData
      (Variables|Default|SetProjectileTargetLocation (.Location (Collision|BreakHitResult (Ability|TargetData|GetHitResultfromTargetData _data))))
      (Variables|Default|SetHit%20Actor (.HitActor (Collision|BreakHitResult (Ability|TargetData|GetHitResultfromTargetData _data))))
      (Class|CombatInterface|SetFacingTarget(Message) (Ability|GetAvatarActorfromActorInfo) (Variables|Default|GetProjectileTargetLocation))
      (|PlayMontageandWaitProxy "None" "/Game/Assets/Characters/Aura/Animations/Abilities/AnimMontages/AM_AuraFireBolt.AM_AuraFireBolt" 1.0 "None" true 1.0 0.0 false
        (:then
          (Ability|Tasks|WaitGameplayEvent "(TagName=\"Event.Montage.Firebolt\")" 0 true
            (:EventReceived
              (Class|AuraFireBolt|SpawnProjectiles (Variables|Default|GetProjectileTargetLocation) (GameplayTags|MakeLiteralGameplayTag "(TagName=\"CombatSocket.Weapon\")") true 2e+01 (Variables|Default|GetHit%20Actor)))))
        (:OnCompleted
          (Ability|EndAbility))))))

(event Ability|EventOnEndAbility
  (params (bWasCancelled :type Boolean)))