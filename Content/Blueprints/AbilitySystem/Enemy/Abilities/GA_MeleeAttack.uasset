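; Enemy melee attack ability that plays a random tagged attack montage from the avatar's combat interface.
; A looping timer keeps the avatar facing its combat target until the ability ends.
; The montage's gameplay event triggers a radius check at the tagged combat socket, damaging live non-friendly players.
; A hit fires the melee gameplay cue and ends the ability immediately; otherwise it ends when the montage finishes or is interrupted.
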(event Custom|OnSetFacingTarget
  (Class|CombatInterface|SetFacingTarget (Variables|Default|GetAs%20Combat%20Interface) (Transformation|GetActorLocation (Variables|Default|GetCombatTarget))))

(event Ability|EventActivateAbility
  (Variables|Default|SetHasHitTarget false)
  (Utilities|FlowControl|Sequence
    (:then_0
      (bind _ascombat_interface (Utilities|Casting|CastToCombatInterface (Ability|GetAvatarActorfromActorInfo)))
      (Variables|Default|SetAs%20Combat%20Interface _ascombat_interface)
      (bind _returnvalue (Class|EnemyInterface|GetCombatTarget(Message) (Ability|GetAvatarActorfromActorInfo)))
      (Variables|Default|SetCombatTarget _returnvalue))
    (:then_1
      (Variables|Default|SetThisTaggedMontage (Class|AuraDamageGameplayAbility|GetRandomTaggedMontagesfromArray (Class|CombatInterface|GetAttackMontages (Variables|Default|GetAs%20Combat%20Interface))))
      (|PlayMontageandWaitProxy "None" (.AttackMontage (Utilities|Struct|BreakTaggedMontages (Variables|Default|GetThisTaggedMontage))) 1.0 "None" true 1.0 0.0 false
        (:then
          (Ability|Tasks|WaitGameplayEvent (.MontageTag (Utilities|Struct|BreakTaggedMontages (Variables|Default|GetThisTaggedMontage))) 0 true
            (:then
              (bind _returnvalue_2 (Utilities|Time|SetTimerbyEvent (delegate Custom|OnSetFacingTarget) 0.016 true))
              (Variables|Default|SetFacingTargetHandle _returnvalue_2))
            (:EventReceived
              (bind _returnvalue_3 (Class|CombatInterface|GetCombatSocketLocation(Message) (Ability|GetAvatarActorfromActorInfo) (.SocketTag (Utilities|Struct|BreakTaggedMontages (Variables|Default|GetThisTaggedMontage)))))
              (Variables|Default|SetCombatSocketLocation _returnvalue_3)
              (bind _outoverlappingactors (Class|AuraAbilitySystemLibrary|GetLivePlayersWithinRadius (Ability|GetAvatarActorfromActorInfo) (Utilities|Array|MakeArray (Ability|GetAvatarActorfromActorInfo)) 5e+01 (Variables|Default|GetCombatSocketLocation)))
              (for _array_element _outoverlappingactors
                (Variables|Default|SetThisOtherTarget _array_element)
                (bind _returnvalue_4 (Class|AuraAbilitySystemLibrary|IsNotFriend (Ability|GetAvatarActorfromActorInfo) (Variables|Default|GetThisOtherTarget)))
                (if _returnvalue_4
                  (Variables|Default|SetHasHitTarget true)
                  (Class|AuraDamageGameplayAbility|CauseDamage (Variables|Default|GetThisOtherTarget))))
              (if (Variables|Default|GetHasHitTarget)
                (Class|GameplayAbility|ExecuteGameplayCuewithParams "(TagName=\"GameplayCue.MeleeAttack\")" (Ability|GameplayCue|MakeGameplayCueParameters :AggregatedSourceTags (GameplayTags|MakeGameplayTagContainerfromTag (.MontageTag (Utilities|Struct|BreakTaggedMontages (Variables|Default|GetThisTaggedMontage)))) :Location (Variables|Default|GetCombatSocketLocation) :EffectCauser (Ability|GetAvatarActorfromActorInfo) :SourceObject (Variables|Default|GetCombatTarget)))
                (Ability|EndAbility)))))
        (:OnCompleted
          (Ability|EndAbility :!label _label))
        (:OnInterrupted
          (goto _label))
        (:OnCancelled
          (goto _label))))))

(event Ability|EventOnEndAbility
  (params (bWasCancelled :type Boolean))
  (Utilities|Time|ClearandInvalidateTimerbyHandle (Variables|Default|GetFacingTargetHandle))
  (Variables|Default|SetHasHitTarget false))