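; Player gameplay ability Arcane Shards: shows a magic circle, then on input press takes the point under the mouse, faces it and plays a cast montage.
; The montage's gameplay event spawns a BP_PointCollection that supplies ground points at a random yaw.
; A looping timer steps through the points, firing a gameplay cue and applying radial damage to nearby live actors, excluding the caster.
; After the last point it clears the timer, destroys the collection and ends.
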(event Custom|SpawnShard
  (CallFunction|SpawnArcaneShards))

(event Ability|EventActivateAbility
  (Utilities|FlowControl|Sequence
    (:then_0
      (Class|PlayerInterface|ShowMagicCircle(Message) (Ability|GetAvatarActorfromActorInfo) 0))
    (:then_1
      (Ability|Tasks|WaitInputPress false
        (:OnPress
          (bind _data (|TargetDataUnderMouse)
            (:ValidData
              (Variables|Default|SetReturn%20Value%20Location (.location (Ability|TargetData|GetHitResultfromTargetData _data)))
              (Variables|Default|SetReturn%20Value%20Impact%20Point (.impactpoint (Ability|TargetData|GetHitResultfromTargetData _data)))
              (CallFunction|FaceSpellLocation)
              (Class|PlayerInterface|HideMagicCircle(Message) (Ability|GetAvatarActorfromActorInfo))
              (|PlayMontageandWaitProxy "None" "/Game/Assets/Characters/Aura/Animations/Abilities/AnimMontages/AM_ArcaneShards.AM_ArcaneShards" 1.0 "None" true 1.0 0.0 false
                (:then
                  (Ability|Tasks|WaitGameplayEvent "(TagName=\"Event.Montage.ArcaneShards\")" 0 true
                    (:EventReceived
                      (bind _returnvalue (Game|SpawnActorfromClass "/Game/Blueprints/Actors/Decals/BP_PointCollection.BP_PointCollection_C" (Math|Transform|MakeTransform (Variables|Default|GetReturn%20Value%20Location) "0, 0, 0" "1.000000,1.000000,1.000000") "Undefined" "MultiplyWithRoot" 0 0))
                      (Variables|Default|SetPointCollection _returnvalue)
                      (Variables|Default|SetLocal_Ground_Points (Class|PointCollection|GetGroundPoints (Variables|Default|GetPointCollection) (Variables|Default|GetReturn%20Value%20Impact%20Point) (Variables|Default|GetNumPoints) (Math|Random|RandomFloatinRange 0.0 3.6e+02)))
                      (bind _returnvalue_2 (Utilities|Time|SetTimerbyEvent (delegate Custom|SpawnShard) 0.15 true))
                      (Variables|Default|SetShardSpawnTimerHandle _returnvalue_2)
                      (CallFunction|SpawnShard))))))))))))

(fn SpawnArcaneShards
  (bind _local_ground_points (Variables|Default|GetLocal_Ground_Points))
  (bind _count (Variables|Default|GetCount))
  (bind _output (Utilities|Array|Get(acopy) _local_ground_points _count))
  (bind _returnvalue (Transformation|GetWorldTransform _output))
  (if (> (Variables|Default|GetNumPoints) (Variables|Default|GetCount))
    (Variables|Default|SetPointLocation (.location _returnvalue))
    (Variables|Default|SetPointRotation (.rotation _returnvalue))
    (Math|Integer|IncrementInt (Variables|Default|GetCount)
      (:%20%20
        (Class|GameplayAbility|ExecuteGameplayCuewithParams "(TagName=\"GameplayCue.ArcaneShards\")" (Ability|GameplayCue|MakeGameplayCueParameters :Location (Variables|Default|GetPointLocation) :Normal (Math|Vector|GetRightVector (Variables|Default|GetPointRotation))))
        (bind _outoverlappingactors (Class|AuraAbilitySystemLibrary|GetLivePlayersWithinRadius (Ability|GetAvatarActorfromActorInfo) (Utilities|Array|MakeArray (Ability|GetAvatarActorfromActorInfo)) (Variables|Default|GetRadialDamageOuterRadius) (Variables|Default|GetPointLocation)))
        (for _array_element _outoverlappingactors
          (Class|AuraAbilitySystemLibrary|ApplyDamageEffect (Class|AuraDamageGameplayAbility|MakeDamageEffectParamsfromClassDefaults _array_element (Variables|Default|GetPointLocation))))))
    (else
      (CallFunction|PreparetoEndAbility)
      (Ability|EndAbility))))

(fn PreparetoEndAbility
  (Utilities|Time|InvalidateTimerHandle (Variables|Default|GetShardSpawnTimerHandle))
  (Variables|Default|SetCount 0)
  (Actor|DestroyActor (Variables|Default|GetPointCollection)))

(fn FaceSpellLocation
  (Class|CombatInterface|SetFacingTarget(Message) (Ability|GetAvatarActorfromActorInfo) (Variables|Default|GetReturn%20Value%20Impact%20Point)))