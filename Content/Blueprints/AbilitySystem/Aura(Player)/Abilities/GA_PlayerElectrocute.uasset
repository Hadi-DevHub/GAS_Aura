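; Player Electrocute gameplay ability: a held-input channeled shock cast toward the point under the mouse cursor.
; On activation it stores the cursor hit, hides the cursor, faces the avatar to the target, fires the ShockBurst cue and plays the montage.
; A montage event starts the shock loop, adds the weapon-attached ShockLoop cue and disables movement.
; Input release restores cursor and walking, removes the loop cue and ends the ability.
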(event Ability|EventActivateAbility
  ;[0.8385 0.4618 0.2833] Store Datas
  (CallFunction|EnforceCombatInterfaceCheck)
  (bind _data (|TargetDataUnderMouse)
    (:ValidData
      (Class|AuraBeamSpell|StoreMouseDataInfo (Ability|TargetData|GetHitResultfromTargetData _data))
      (Class|AuraBeamSpell|StoreOwnerPlayerController)
      (Utilities|FlowControl|Sequence
        (:then_0
          (Variables|/Script/Engine.PlayerController|SetbShowMouseCursor (Variables|Default|GetStoredOwnerPlayerController) false)
          (CallFunction|SetFacingTarget)
          ;[0.1583 0.1677 0.1979] Comment
          (GameplayCue|ExecuteGameplayCue :GameplayCueTag "(TagName=\"GameplayCue.ShockBurst\")")
          (|PlayMontageandWaitProxy "None" (Variables|Default|GetElectrocuteMontage) 1.0 "None" true 1.0 0.0 false
            (:then
              (Ability|Tasks|WaitGameplayEvent "(TagName=\"Event.Montage.Electrocute\")" 0 true
                (:EventReceived
                  (Class|CombatInterface|SetinShockLoop(Message) (Variables|Default|GetStoredOwnerAvatar) true)
                  (bind _returnvalue (Class|CombatInterface|GetWeapon(Message) (Ability|GetAvatarActorfromActorInfo)))
                  (GameplayCue|AddGameplayCueOnActor(Looping) (Ability|GetAvatarActorfromActorInfo) "(TagName=\"GameplayCue.ShockLoop\")" (Ability|GameplayCue|MakeGameplayCueParameters :Location (Variables|Default|GetStoredHitLocation) :TargetAttachComponent _returnvalue))
                  (Pawn|Components|CharacterMovement|DisableMovement (Variables|/Script/Engine.Character|GetCharacterMovement (Variables|Default|GetStoredOwnerAvatar))))))))
        (:then_1
          (Ability|Tasks|WaitInputRelease false
            (:OnRelease
              (CallFunction|EndingtheAbility)
              (Ability|EndAbility))))))))

(fn EnforceCombatInterfaceCheck
  (if (not (Utilities|DoesObjectImplementInterface (Ability|GetAvatarActorfromActorInfo) "/Script/Aura.CombatInterface"))
    (Ability|EndAbility)))

(fn EndingtheAbility
  (Variables|/Script/Engine.PlayerController|SetbShowMouseCursor (Variables|Default|GetStoredOwnerPlayerController) true)
  (Class|CombatInterface|SetinShockLoop(Message) (Variables|Default|GetStoredOwnerAvatar) false)
  (Pawn|Components|CharacterMovement|SetMovementMode (Variables|/Script/Engine.Character|GetCharacterMovement (Variables|Default|GetStoredOwnerAvatar)) "MOVE_Walking" 0)
  (GameplayCue|RemoveGameplayCue "(TagName=\"GameplayCue.ShockLoop\")"))

(fn SetFacingTarget
  (Class|CombatInterface|SetFacingTarget(Message) (Ability|GetAvatarActorfromActorInfo) (Variables|Default|GetStoredHitLocation)))