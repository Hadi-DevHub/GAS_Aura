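; Melee attack gameplay ability that plays the avatar's attack montage while turning it toward its combat target.
; The avatar supplies montage and target through CombatInterface, and a looping near-per-frame timer updates facing until the ability ends.
; A montage gameplay event currently only draws a debug sphere at the combat socket, with no damage applied.
; The ability ends when the montage completes, is interrupted or is cancelled.
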(event Custom|OnSetFacingTarget
  (Class|CombatInterface|SetFacingTarget (Variables|Default|GetAs%20Combat%20Interface) (Transformation|GetActorLocation (Variables|Default|GetCombatTarget))))

(event Ability|EventActivateAbility
  (Utilities|FlowControl|Sequence
    (:then_0
      (bind _ascombat_interface (Utilities|Casting|CastToCombatInterface (Ability|GetAvatarActorfromActorInfo)))
      (Variables|Default|SetAs%20Combat%20Interface _ascombat_interface)
      (bind _returnvalue (Class|EnemyInterface|GetCombatTarget(Message) (Ability|GetAvatarActorfromActorInfo)))
      (Variables|Default|SetCombatTarget _returnvalue))
    (:then_1
      (bind _returnvalue_2 (Class|CombatInterface|GetAttackMontage (Variables|Default|GetAs%20Combat%20Interface)))
      (|PlayMontageandWaitProxy "None" _returnvalue_2 1.0 "None" true 1.0 0.0 false
        (:then
          (Ability|Tasks|WaitGameplayEvent "(TagName=\"Event.Montage.MeleeAttack\")" 0 true
            (:then
              (bind _returnvalue_3 (Utilities|Time|SetTimerbyEvent (delegate Custom|OnSetFacingTarget) 0.016 true))
              (Variables|Default|SetFacingTargetHandle _returnvalue_3))
            (:EventReceived
              (bind _returnvalue_4 (Class|CombatInterface|GetCombatSocketLocation(Message) (Ability|GetAvatarActorfromActorInfo)))
              (Rendering|Debug|DrawDebugSphere _returnvalue_4 4e+01 12 "(R=0.000000,G=0.014535,B=1.000000,A=1.000000)" 1.0 1.0))))
        (:OnCompleted
          (Ability|EndAbility :!label _label))
        (:OnInterrupted
          (goto _label))
        (:OnCancelled
          (goto _label))))))

(event Ability|EventOnEndAbility
  (params (bWasCancelled :type Boolean))
  (Utilities|Time|ClearandInvalidateTimerbyHandle (Variables|Default|GetFacingTargetHandle)))