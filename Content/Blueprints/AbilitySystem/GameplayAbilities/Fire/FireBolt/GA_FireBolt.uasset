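; GA_FireBolt is the gameplay ability that casts the Fire Bolt projectile spell.
; On activation it gets target data under the mouse and turns the avatar toward the hit location through the CombatInterface.
; It plays the Aura fire bolt montage, waits once for that montage's Firebolt gameplay event, spawns the projectile at the target, then ends after a short delay.
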(event Ability|EventActivateAbility
  (bind _data (|TargetDataUnderMouse)
    (:ValidData
      (Variables|Default|SetProjectileTargetLocation (.Location (Collision|BreakHitResult (Ability|TargetData|GetHitResultfromTargetData _data))))
      (bind _ascombat_interface (Utilities|Casting|CastToCombatInterface (Ability|GetAvatarActorfromActorInfo)))
      (Class|CombatInterface|SetFacingTarget _ascombat_interface (Variables|Default|GetProjectileTargetLocation))
      (|PlayMontageandWaitProxy "None" "/Game/Assets/Characters/Aura/Animations/Abilities/AnimMontages/AM_AuraFireBolt.AM_AuraFireBolt" 1.0 "None" true 1.0 0.0 false
        (:then
          (Ability|Tasks|WaitGameplayEvent "(TagName=\"Event.Montage.Firebolt\")" 0 true
            (:EventReceived
              (Class|AuraProjectileSpell|SpawnProjectile (Variables|Default|GetProjectileTargetLocation))
              (Utilities|FlowControl|Delay 0.5)
              (Ability|EndAbility))))))))

(event Ability|EventOnEndAbility
  (params (bWasCancelled :type Boolean)))