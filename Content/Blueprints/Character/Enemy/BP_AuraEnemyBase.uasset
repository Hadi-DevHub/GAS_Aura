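; Base enemy Blueprint that handles spawn scale-in, facing, death-style dissolve visuals and loot drops.
; A timeline scales the mesh on BeginPlay, Motion Warping updates the FaceTarget location, and separate timelines drive the Dissolve parameter on character and weapon materials.
; SpawnLoot gets items from loot tiers and evenly spaced rotators, then a looping timer staggers their spawning at random distances around the enemy.
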(event Custom|GenerateLoot
  (if (< (Variables|Default|GetIndex) (- (Variables|Default|GetNumLoot) 1))
    (Game|SpawnActorfromClass (.lootclass (Utilities|Array|Get(acopy) (Variables|Default|GetLootItems) (Variables|Default|GetIndex))) (Math|Conversions|ToTransform(Vector) (+ (* (Math|Vector|GetForwardVector (Utilities|Array|Get(acopy) (Variables|Default|GetSpawnRotators) (Variables|Default|GetIndex))) (Math|Random|RandomFloatinRange (Variables|Default|GetMin%20Dist) (Variables|Default|GetMax%20Dist))) (Transformation|GetActorLocation))) "AdjustIfPossibleButAlwaysSpawn" "MultiplyWithRoot" 0 0)
    (Math|Integer|IncrementInt (Variables|Default|GetIndex))
    (else
      (Utilities|Time|ClearandInvalidateTimerbyHandle (Variables|Default|GetSpawnLootTimerHandle)))))

(event EventSetFacingTarget
  (params (Direction :type Vector%20%28by%20ref%29 :default "0, 0, 0"))
  (Class|MotionWarpingComponent|AddorUpdateWarpTargetfromLocation (Variables|Default|GetMotionWarping) "FaceTarget" Direction))

(event EventBeginPlay
  (bind _scaletimeline (Timeline|SpawnTimeline Play)
    (:Update
      (Transformation|SetRelativeScale3D (Variables|Character|GetMesh) (Math|Vector|MakeVector _scaletimeline _scaletimeline _scaletimeline)))))

(event EventSpawnLoot
  (bind _returnvalue (Class|AuraAbilitySystemLibrary|GetLootTiers))
  (Utilities|IsValid _returnvalue
    (:Is%20Valid
      (bind _returnvalue_2 (Class|LootTiers|GetLootItems _returnvalue))
      (bind _output_get (Variables|Default|SetLootItems _returnvalue_2))
      (Variables|Default|SetNumLoot (Utilities|Array|Length _output_get))
      (bind _returnvalue_3 (Class|AuraAbilitySystemLibrary|EvenlySpacedRotators (Math|Vector|GetForwardVector (Transformation|GetActorRotation)) (Math|Vector|VectorUp) (Variables|Default|GetLootSpawnSpreadAngle) (Variables|Default|GetNumLoot)))
      (Variables|Default|SetSpawnRotators _returnvalue_3)
      (Variables|Default|SetIndex 0)
      (bind _returnvalue_4 (Utilities|Time|SetTimerbyEvent (delegate Custom|GenerateLoot) 0.1 true))
      (Variables|Default|SetSpawnLootTimerHandle _returnvalue_4)
      (CallFunction|GenerateLoot))))

(event EventStartCharacterDissolveTimeline
  (params (DynamicMaterialInstance :type Material%20Instance%20Dynamic%20Object%20Reference))
  (bind _dissolve (Timeline|CharacterDissolveTimeline Play)
    (:Update
      (Rendering|Material|SetScalarParameterValue DynamicMaterialInstance "Dissolve" _dissolve :!class /Script/Engine.MaterialInstanceDynamic))))

(event EventStartWeaponDissolveTimeline
  (params (DynamicMaterialInstance :type Material%20Instance%20Dynamic%20Object%20Reference))
  (bind _dissolve (Timeline|WeaponDissolveTimeline Play)
    (:Update
      (Rendering|Material|SetScalarParameterValue DynamicMaterialInstance "Dissolve" _dissolve :!class /Script/Engine.MaterialInstanceDynamic))))

(fn ConstructionScript)