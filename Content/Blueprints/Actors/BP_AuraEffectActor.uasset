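; Base effect actor that animates itself like dropped loot when it spawns.
; On BeginPlay, the LootDropCurve timeline drives a jump height scaled by SpawnApex and a uniform scale.
; When the timeline finishes, it calls StartSinusoidalMovement and StartRotation, which are defined outside this graph.
; Tick applies CalculatedLocation and CalculatedRotation to the actor every frame, without sweep.
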(event EventTick
  (params (DeltaSeconds :type Float%20%28single-precision%29))
  (Transformation|SetActorLocation (Variables|Default|GetCalculatedLocation) false false)
  (Transformation|SetActorRotation (Variables|Default|GetCalculatedRotation)))

(event EventBeginPlay
  (bind _initiallocation (Variables|Default|GetInitialLocation))
  (bind (_direction _jumptrack _scaletrack) (Timeline|LootDropCurve Play)
    (:Update
      (Variables|Default|SetCalculatedLocation (Math|Vector|MakeVector (.x _initiallocation) (.y _initiallocation) (+ (.z _initiallocation) (* _jumptrack (Variables|Default|GetSpawnApex)))))
      (Transformation|SetActorScale3D (Math|Vector|MakeVector _scaletrack _scaletrack _scaletrack)))
    (:Finished
      (Class|AuraActorEffect|StartSinusoidalMovement)
      (Class|AuraActorEffect|StartRotation))))

(fn ConstructionScript)