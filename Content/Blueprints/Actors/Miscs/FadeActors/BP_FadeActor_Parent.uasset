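; Parent actor for meshes that fade out and back in on request, toggling whether they block traces.
; The construction script caches the mesh's default materials and builds dynamic instances from a configured material list.
; FadeOut swaps in those instances and plays a timeline driving their Fade parameter; Fadein reverses it.
; On finish, full fade scale restores default materials and blocking, while zero ignores Visibility and a custom trace channel.
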(event EventFadeOut
  (CallFunction|SetMaterialtoDynamicMaterialInstance)
  (bind _fadescale (Timeline|Timeline Play)
    (:Update
      (for _array_element (Variables|Default|GetDynamicMaterialInstances)
        (Rendering|Material|SetScalarParameterValue _array_element "Fade" _fadescale :!class /Script/Engine.MaterialInstanceDynamic)))
    (:Finished
      (CallFunction|OnFadeTimelineFinished _fadescale))))

(event EventFadein
  (bind _fadescale (Timeline|Timeline Reverse)
    (:Update
      (for _array_element (Variables|Default|GetDynamicMaterialInstances)
        (Rendering|Material|SetScalarParameterValue _array_element "Fade" _fadescale :!class /Script/Engine.MaterialInstanceDynamic)))
    (:Finished
      (CallFunction|OnFadeTimelineFinished _fadescale))))

(fn ConstructionScript
  (CallFunction|StoreDefaultandInstancedMaterials))

(fn StoreDefaultandInstancedMaterials
  (Variables|Default|SetDefaultMaterials (Rendering|Material|GetMaterials (Variables|Default|GetMesh)))
  (for _array_element (Variables|Default|GetMaterialInstances)
    (bind _returnvalue (Rendering|Material|CreateDynamicMaterialInstance _array_element "None" "None" :!class /Script/Engine.KismetMaterialLibrary))
    (Utilities|Array|AddUnique (Variables|Default|GetDynamicMaterialInstances) _returnvalue)))

(fn SetMaterialtoDynamicMaterialInstance
  (for (_array_element _array_index) (Variables|Default|GetDynamicMaterialInstances)
    (Rendering|Material|SetMaterial (Variables|Default|GetMesh) _array_index _array_element)))

(fn SettoDefaultMaterial
  (for (_array_element _array_index) (Variables|Default|GetDefaultMaterials)
    (Rendering|Material|SetMaterial (Variables|Default|GetMesh) _array_index _array_element)))

(fn OnFadeTimelineFinished
  (params (FadeScale :type Float%20%28double-precision%29))
  (if (>= FadeScale 1.0)
    (CallFunction|SettoDefaultMaterial)
    (Collision|SetCollisionResponsetoChannel (Variables|Default|GetMesh) "ECC_GameTraceChannel2" "ECR_Block")
    (Collision|SetCollisionResponsetoChannel (Variables|Default|GetMesh) "ECC_Visibility" "ECR_Block")
    (elif (<= FadeScale 0.0)
      (Collision|SetCollisionResponsetoChannel (Variables|Default|GetMesh) "ECC_GameTraceChannel2" "ECR_Ignore")
      (CallFunction|SetMaterialtoDynamicMaterialInstance)
      (Collision|SetCollisionResponsetoChannel (Variables|Default|GetMesh) "ECC_Visibility" "ECR_Ignore"))))